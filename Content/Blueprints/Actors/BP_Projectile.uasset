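; BP_Projectile is a projectile actor that handles the trail and explosion effects, with trail color keyed to ControllerIndex.
; Shortly after BeginPlay it attaches a trail emitter to its mesh and tints it through a color parameter for indices 0 to 3.
; On Destroyed it spawns an explosion, plays a sound and triggers a world camera shake.
; An unwired node for ignoring the instigator during movement never runs.
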(event `self.ReceiveBeginPlay`
  (`KismetSystemLibrary.Delay` 0.05)
  (bind _returnvalue (`GameplayStatics.SpawnEmitterAttached` "/Game/Particles/P_ProjectileTrail.P_ProjectileTrail" (`self.StMesh`) "None" (`self.K2_GetActorLocation` self) (struct) (`self.Scale`) "KeepWorldPosition"))
  (switch `int` (`self.ControllerIndex`)
    (:`0`
      (`FXSystemComponent.SetColorParameter` _returnvalue "ProjColor" (struct :`G` 0.08272 :`B` 0.421875 :`A` 1.0)))
    (:`1`
      (`FXSystemComponent.SetColorParameter` _returnvalue "ProjColor" (struct :`R` 0.526042 :`G` 0.212 :`A` 1.0)))
    (:`2`
      (`FXSystemComponent.SetColorParameter` _returnvalue "ProjColor" (struct :`R` 0.94902 :`G` 0.007843 :`B` 0.4 :`A` 1.0)))
    (:`3`
      (`FXSystemComponent.SetColorParameter` _returnvalue "ProjColor" (struct :`G` 0.196078 :`B` 0.047059 :`A` 1.0)))))

(event `self.ReceiveDestroyed`
  (bind _returnvalue (`self.K2_GetActorLocation` self))
  (`GameplayStatics.SpawnEmitterAtLocation` "/Game/Particles/P_Explosion.P_Explosion" _returnvalue (struct) (2.0 2.0 2.0))
  (`GameplayStatics.PlaySoundAtLocation` "/Game/Audio/SoundCues/ExplosionSoundCue.ExplosionSoundCue" _returnvalue (struct) 0.6 1.0 0.0 null null null)
  (`GameplayStatics.PlayWorldCameraShake` "/Game/Blueprints/Actors/BP_CameraShake.BP_CameraShake_C" (`self.K2_GetActorLocation`) 0.0 20000.0))

(fn `UserConstructionScript`)