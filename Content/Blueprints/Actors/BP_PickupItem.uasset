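; Pickup item actor for the Mayhaemsters game mode, representing one of eight item types such as shield, speed changers, map resetter and jammer.
; SetItemMesh turns the mesh toward the player camera once, then applies the mesh, trigger extent and any offset, rotation or scale for its ItemType.
; On destruction it marks its ItemIndex spawn point available again in the game mode.
; An up-and-down bobbing timeline exists but never runs.
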(event `self.ReceiveDestroyed`
  (`KismetArrayLibrary.Array_Set` (`/Game/Blueprints/Game/BP_GM_Mayhaemsters.SpawnPointAvailability` (cast `/Game/Blueprints/Game/BP_GM_Mayhaemsters` (`GameplayStatics.GetGameMode`) :!pure true)) (`self.ItemIndex`) true))

(fn `FaceCamera`
  (`SceneComponent.K2_SetWorldRotation` (`self.StMesh`) (`KismetMathLibrary.FindLookAtRotation` (`SceneComponent.K2_GetComponentLocation` (`self.StMesh`)) (`self.K2_GetActorLocation` (`GameplayStatics.GetPlayerCameraManager` 0))) false false))

(fn `Set Item Mesh`
  (`self.FaceCamera`)
  (switch `EPickupItemType` (`self.ItemType`)
    (:`Remapper`
      (`StaticMeshComponent.SetStaticMesh` (`self.StMesh`) "/Game/Meshes/StaticMeshes/Items/remap.remap")
      (`SceneComponent.K2_AddLocalOffset` (`self.StMesh`) (50.0 -50.0 0.0) false false)
      (`BoxComponent.SetBoxExtent` (`self.BoxTrigger`) (150.0 150.0 150.0) true)
      (`self.SetActorScale3D` (0.4 0.4 0.4)))
    (:`Shield`
      (`StaticMeshComponent.SetStaticMesh` (`self.StMesh`) "/Game/Meshes/StaticMeshes/Items/StM_Item_Shield.StM_Item_Shield")
      (`SceneComponent.K2_AddLocalOffset` (`self.StMesh`) (50.0 -50.0 0.0) false false)
      (`BoxComponent.SetBoxExtent` (`self.BoxTrigger`) (50.0 50.0 50.0) true))
    (:`SpeedUp`
      (`StaticMeshComponent.SetStaticMesh` (`self.StMesh`) "/Game/Meshes/StaticMeshes/Items/StM_Item_SpeedUp.StM_Item_SpeedUp")
      (`SceneComponent.K2_AddLocalOffset` (`self.StMesh`) (50.0 75.0 0.0) false false)
      (`BoxComponent.SetBoxExtent` (`self.BoxTrigger`) (20.0 50.0 100.0) true)
      (`SceneComponent.K2_AddRelativeRotation` (`self.StMesh`) (struct :`Roll` -90.0) false false))
    (:`SpeedDown`
      (`StaticMeshComponent.SetStaticMesh` (`self.StMesh`) "/Game/Meshes/StaticMeshes/Items/StM_Item_SpeedDown.StM_Item_SpeedDown")
      (`BoxComponent.SetBoxExtent` (`self.BoxTrigger`) (20.0 50.0 100.0) true)
      (`SceneComponent.K2_AddRelativeRotation` (`self.StMesh`) (struct :`Yaw` 20.0 :`Roll` -90.0) false false))
    (:`MapResetter`
      (`StaticMeshComponent.SetStaticMesh` (`self.StMesh`) "/Game/Meshes/StaticMeshes/Items/StM_Item_ResetMap.StM_Item_ResetMap")
      (`SceneComponent.K2_AddLocalOffset` (`self.StMesh`) (-150.0 0.0 0.0) false false)
      (`BoxComponent.SetBoxExtent` (`self.BoxTrigger`) (20.0 100.0 75.0) true)
      (`SceneComponent.K2_AddRelativeRotation` (`self.StMesh`) (struct :`Yaw` 270.0) false false))
    (:`Mystery`
      (`StaticMeshComponent.SetStaticMesh` (`self.StMesh`) "/Game/Meshes/StaticMeshes/Items/mystery.mystery")
      (`SceneComponent.K2_AddLocalOffset` (`self.StMesh`) (0.0 50.0 0.0) false false)
      (`BoxComponent.SetBoxExtent` (`self.BoxTrigger`) (100.0 100.0 100.0) true)
      (`self.SetActorScale3D` (0.35 0.35 0.35)))
    (:`Unifier`
      (`StaticMeshComponent.SetStaticMesh` (`self.StMesh`) "/Game/Meshes/StaticMeshes/Items/unifier.unifier")
      (`SceneComponent.K2_AddLocalOffset` (`self.StMesh`) (0.0 50.0 0.0) false false)
      (`BoxComponent.SetBoxExtent` (`self.BoxTrigger`) (100.0 100.0 100.0) true)
      (`self.SetActorScale3D` (0.27 0.27 0.27)))
    (:`Jammer`
      (`StaticMeshComponent.SetStaticMesh` (`self.StMesh`) "/Game/Meshes/StaticMeshes/Items/jammer.jammer")
      (`SceneComponent.K2_AddLocalOffset` (`self.StMesh`) (0.0 50.0 0.0) false false)
      (`BoxComponent.SetBoxExtent` (`self.BoxTrigger`) (100.0 100.0 100.0) true)
      (`self.SetActorScale3D` (0.31 0.31 0.31))))
  (`SceneComponent.K2_AddRelativeRotation` (`self.StMesh`) (struct :`Pitch` 90.0) false false))

(fn `UserConstructionScript`)