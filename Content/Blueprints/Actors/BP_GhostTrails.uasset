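; BP_GhostTrails is a short-lived afterimage actor that shows a fading ghost of the player character's pose.
; On BeginPlay it gets the player pawn and gives each Ghost mesh material slot a dynamic instance of M_GhostTrails_Inst.
; The Ghost copies the pose from the player's mesh as a frozen snapshot.
; An Opacity timeline drives the Opacity parameter on those materials, then destroys the actor when finished.
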(event `self.ReceiveBeginPlay`
  (bind _asbp_ch_player (cast `/Game/Blueprints/Characters/BP_Ch_Player` (`GameplayStatics.GetPlayerPawn` 0)))
  (set `self.PlayerCharacterRef` _asbp_ch_player)
  (`self.GhostTrails`))

(event `GhostTrails`
  (for _ (`MeshComponent.GetMaterials` (`self.Ghost`))
    (bind _returnvalue (`KismetMaterialLibrary.CreateDynamicMaterialInstance` "/Game/Meshes/SkeletalMeshes/Hamster/Materials/M_GhostTrails_Inst.M_GhostTrails_Inst"))
    (bind _returnvalue_2 (`KismetArrayLibrary.Array_Add` (`self.DynamicMaterials`) _returnvalue))
    (`PrimitiveComponent.SetMaterial` (`self.Ghost`) _returnvalue_2 _returnvalue)
    (`PoseableMeshComponent.CopyPoseFromSkeletalComponent` (`self.Ghost`) (`Character.Mesh` (`self.PlayerCharacterRef`)))
    (bind (_direction _opacity) (`Timeline|Opacity` :!via `PlayFromStart`)
      (:`Update`
        (for _array_element (`self.DynamicMaterials`)
          (`MaterialInstanceDynamic.SetScalarParameterValue` _array_element "Opacity" _opacity)))
      (:`Finished`
        (`self.K2_DestroyActor`)))))

(fn `UserConstructionScript`)