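; BP_Morphable is an actor whose skeletal mesh switches between a morphed, non-colliding state and its solid base shape.
; It starts morphed, with the Sphere and Cube_001 morph targets fully applied.
; MorphMesh reverses the Morph timeline to restore the base shape and collision.
; The Mayhaemsters game state's OnMapReset event plays the timeline forward after a delay, disabling collision again.
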(event `self.ReceiveBeginPlay`
  (bind _morphablemesh (`self.MorphableMesh`))
  (`KismetSystemLibrary.Delay` 0.01)
  (`|ExecutionSequence`
    (:`then_0`
      (`SkeletalMeshComponent.SetMorphTarget` _morphablemesh "Sphere" 1.0 true)
      (`SkeletalMeshComponent.SetMorphTarget` _morphablemesh "Cube_001" 1.0 true)
      (`PrimitiveComponent.SetCollisionEnabled` _morphablemesh "NoCollision")
      (set `self.bMorphed` true))
    (:`then_1`
      (add `C_GS_Mayhaemsters.OnMapReset` (cast `/Game/Blueprints/Game/BP_GS_Mayhaemsters` (`GameplayStatics.GetGameState`) :!pure true) (delegate `ResetMorphState`)))))

(event `ResetMorphState`
  (bind _morphablemesh (`self.MorphableMesh`))
  (bind _morphablemesh_2 (`self.MorphableMesh`))
  (if (not (`self.bMorphed`))
    (`KismetSystemLibrary.Delay` 1.0)
    (bind (_direction _alpha) (`Timeline|Morph` :!via `PlayFromStart` :!label _label)
      (:`Update`
        (`SkeletalMeshComponent.SetMorphTarget` _morphablemesh_2 "Sphere" _alpha true)
        (`SkeletalMeshComponent.SetMorphTarget` _morphablemesh_2 "Cube_001" _alpha true))
      (:`Finished`
        (if (`|EnumEquality` _direction "Forward")
          (`PrimitiveComponent.SetCollisionEnabled` _morphablemesh "NoCollision")
          (set `self.bMorphed` true)
          (else
            (`PrimitiveComponent.SetCollisionEnabled` _morphablemesh "QueryAndPhysics")))))))

(event `self.MorphMesh`
  (if (`self.bMorphed`)
    (set `self.bMorphed` false)
    (goto _label :!via `ReverseFromEnd`)))

(fn `UserConstructionScript`
  (`SkinnedMeshComponent.SetSkinnedAssetAndUpdate` (`self.MorphableMesh`) (`self.MorphTarget`) true))