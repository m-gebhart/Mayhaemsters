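; BP_WaterActor is a water prop actor that can appear as a boat, buoy or barrel.
; Its construction script switches on WaterObjectType to set the static mesh and its relative scale.
; The boat and buoy share one larger scale, while the barrel uses a smaller one.
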(fn `UserConstructionScript`
  (switch `EWaterObjectType` (`self.WaterObjectType`)
    (:`Boat`
      (`StaticMeshComponent.SetStaticMesh` (`self.StaticMesh`) "/Game/Meshes/StaticMeshes/WaterObjects/Boat.Boat")
      (`SceneComponent.SetRelativeScale3D` (`self.StaticMesh`) (2.15 2.15 2.15) :!label _label))
    (:`Buoy`
      (`StaticMeshComponent.SetStaticMesh` (`self.StaticMesh`) "/Game/Meshes/StaticMeshes/WaterObjects/Buoy.Buoy")
      (goto _label))
    (:`Barrel`
      (`StaticMeshComponent.SetStaticMesh` (`self.StaticMesh`) "/Game/Meshes/StaticMeshes/WaterObjects/Barrel.Barrel")
      (`SceneComponent.SetRelativeScale3D` (`self.StaticMesh`) (0.9 0.9 0.9)))))