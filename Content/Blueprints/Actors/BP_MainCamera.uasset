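; Shared arena camera for two to four players that frames the group and kills players who stay off screen too long.
; Each tick it eases toward the clamped average player position, rotates to look at it, and zooms the spring arm by the largest inter-player distance.
; A looping timer projects each player to screen, flags those outside the viewport, and self-destructs them after the game mode's border death delay unless they return.
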(event `CheckPlayersInArena`
  (bind _player4 (`self.Player4`))
  (bind _player1 (`self.Player1`))
  (bind _player2 (`self.Player2`))
  (bind _player3 (`self.Player3`))
  (`|ExecutionSequence`
    (:`then_0`
      (bind _isonscreen (`self.PlayerCamVisibilityCheck` 0))
      (if _isonscreen
        (`/Engine/EditorBlueprintResources/StandardMacros.DoOnce` false :!label _label
          (:`Completed`
            (bind _output_get (set `self.P1Outside` false))
            (set `/Game/Blueprints/Characters/BP_Ch_Player.bOutOfCamera` _output_get (`self.Player1`))
            (goto _label_2 :!via `Reset`)))
        (else
          (`|ExecutionSequence`
            (:`then_0`
              (goto _label :!via `Reset`))
            (:`then_1`
              (`/Engine/EditorBlueprintResources/StandardMacros.DoOnce` false :!label _label_2
                (:`Completed`
                  (bind _output_get_2 (set `self.P1Outside` true))
                  (`/Engine/EditorBlueprintResources/StandardMacros.IsValid` _player1
                    (:`Is Valid`
                      (set `/Game/Blueprints/Characters/BP_Ch_Player.bOutOfCamera` _output_get_2 _player1)
                      (`KismetSystemLibrary.RetriggerableDelay` (`self.CameraBorderDeathDuration`))
                      (if (`self.P1Outside`)
                        (`/Engine/EditorBlueprintResources/StandardMacros.IsValid` _player1
                          (:`Is Valid`
                            (`C_Ch_Player.SelfDestruct` _player1)))))))))))))
    (:`then_1`
      (bind _isonscreen_2 (`self.PlayerCamVisibilityCheck` 1))
      (if _isonscreen_2
        (`/Engine/EditorBlueprintResources/StandardMacros.DoOnce` false :!label _label_3
          (:`Completed`
            (bind _output_get_3 (set `self.P2Outside` false))
            (set `/Game/Blueprints/Characters/BP_Ch_Player.bOutOfCamera` _output_get_3 (`self.Player2`))
            (goto _label_4 :!via `Reset`)))
        (else
          (`|ExecutionSequence`
            (:`then_0`
              (goto _label_3 :!via `Reset`))
            (:`then_1`
              (`/Engine/EditorBlueprintResources/StandardMacros.DoOnce` false :!label _label_4
                (:`Completed`
                  (bind _output_get_4 (set `self.P2Outside` true))
                  (`/Engine/EditorBlueprintResources/StandardMacros.IsValid` _player2
                    (:`Is Valid`
                      (set `/Game/Blueprints/Characters/BP_Ch_Player.bOutOfCamera` _output_get_4 _player2)
                      (`KismetSystemLibrary.RetriggerableDelay` (`self.CameraBorderDeathDuration`))
                      (if (`self.P2Outside`)
                        (`/Engine/EditorBlueprintResources/StandardMacros.IsValid` _player2
                          (:`Is Valid`
                            (`C_Ch_Player.SelfDestruct` _player2)))))))))))))
    (:`then_2`
      (bind _isonscreen_3 (`self.PlayerCamVisibilityCheck` 2))
      (if _isonscreen_3
        (`/Engine/EditorBlueprintResources/StandardMacros.DoOnce` false :!label _label_5
          (:`Completed`
            (bind _output_get_5 (set `self.P3Outside` false))
            (set `/Game/Blueprints/Characters/BP_Ch_Player.bOutOfCamera` _output_get_5 (`self.Player3`))
            (goto _label_6 :!via `Reset`)))
        (else
          (`|ExecutionSequence`
            (:`then_0`
              (goto _label_5 :!via `Reset`))
            (:`then_1`
              (`/Engine/EditorBlueprintResources/StandardMacros.DoOnce` false :!label _label_6
                (:`Completed`
                  (bind _output_get_6 (set `self.P3Outside` true))
                  (`/Engine/EditorBlueprintResources/StandardMacros.IsValid` _player3
                    (:`Is Valid`
                      (set `/Game/Blueprints/Characters/BP_Ch_Player.bOutOfCamera` _output_get_6 _player3)
                      (`KismetSystemLibrary.RetriggerableDelay` (`self.CameraBorderDeathDuration`))
                      (if (`self.P3Outside`)
                        (`/Engine/EditorBlueprintResources/StandardMacros.IsValid` _player3
                          (:`Is Valid`
                            (`C_Ch_Player.SelfDestruct` _player3)))))))))))))
    (:`then_3`
      (bind _isonscreen_4 (`self.PlayerCamVisibilityCheck` 3))
      (if _isonscreen_4
        (`/Engine/EditorBlueprintResources/StandardMacros.DoOnce` false :!label _label_7
          (:`Completed`
            (bind _output_get_7 (set `self.P4Outside` false))
            (set `/Game/Blueprints/Characters/BP_Ch_Player.bOutOfCamera` _output_get_7 (`self.Player4`))
            (goto _label_8 :!via `Reset`)))
        (else
          (`|ExecutionSequence`
            (:`then_0`
              (goto _label_7 :!via `Reset`))
            (:`then_1`
              (`/Engine/EditorBlueprintResources/StandardMacros.DoOnce` false :!label _label_8
                (:`Completed`
                  (bind _output_get_8 (set `self.P4Outside` true))
                  (`/Engine/EditorBlueprintResources/StandardMacros.IsValid` _player4
                    (:`Is Valid`
                      (set `/Game/Blueprints/Characters/BP_Ch_Player.bOutOfCamera` _output_get_8 _player4)
                      (`KismetSystemLibrary.RetriggerableDelay` (`self.CameraBorderDeathDuration`))
                      (if (`self.P4Outside`)
                        (`/Engine/EditorBlueprintResources/StandardMacros.IsValid` _player4
                          (:`Is Valid`
                            (`C_Ch_Player.SelfDestruct` _player4)))))))))))))))

(event `self.ReceiveBeginPlay`
  (`|ExecutionSequence`
    (:`then_0`
      (`KismetSystemLibrary.K2_SetTimerDelegate` (delegate `CheckPlayersInArena`) 0.5 true)
      (`self.K2_SetActorLocation` (`self.StartPos`))
      (set `SpringArmComponent.TargetArmLength` (`self.StartSpringArmLength`) (`self.SpringArm`))
      (cast `/Game/Blueprints/Game/BP_GI_Mayhaemsters` (`GameplayStatics.GetGameInstance`))
      (`KismetSystemLibrary.Delay` 0.05)
      (`self.GetPlayersReferences`)
      (`self.SetActorTickEnabled` true))
    (:`then_1`
      (set `self.CameraBorderDeathDuration` (`C_GM_Mayhaemsters.CameraBorderDeathDuration` (cast `/Game/Blueprints/Game/BP_GM_Mayhaemsters` (`GameplayStatics.GetGameMode`) :!pure true))))))

(event `self.ReceiveTick`
  (params (DeltaSeconds :type "Float (single-precision)"))
  (switch `int` (`self.PlayerCount`)
    (:`2`
      (`self.SetSpringArmLength2P`)
      (`self.SetCameraTransform2P`))
    (:`3`
      (`self.SetSpringArmLength3P`)
      (`self.SetCameraTransform3P`))
    (:`4`
      (`self.SetSpringArmLength4P`)
      (`self.SetCameraTransform4P`))))

(fn `GetPlayersReferences`
  (bind _outactors (`GameplayStatics.GetAllActorsOfClass` "/Game/Blueprints/Characters/BP_Ch_Player.BP_Ch_Player_C"))
  (set `self.PlayersReferences` _outactors)
  (bind _outactors_2 (`GameplayStatics.GetAllActorsOfClass` "/Script/Engine.PlayerController"))
  (`PlayerController.SetViewTargetWithBlend` _outactors_2 self 0.0 "VTBlend_Linear" 0.0 false)
  (for (_array_element _array_index) (`self.PlayersReferences`)
    (set `self.PlayerIndex` _array_index)
    (switch `int` _array_index
      (:`0`
        (set `self.Player1` _array_element)
        (set `self.PlayerCount` 1))
      (:`1`
        (set `self.Player2` _array_element)
        (set `self.PlayerCount` 2))
      (:`2`
        (set `self.Player3` _array_element)
        (set `self.PlayerCount` 3))
      (:`3`
        (set `self.Player4` _array_element)
        (set `self.PlayerCount` 4)))))

(fn `PlayerCamVisibilityCheck`
  (params (PlayerIndex :type Integer))
  (returns (IsOnScreen :type Boolean))
  (bind _returnvalue (`GameplayStatics.GetPlayerController` PlayerIndex))
  (bind (_returnvalue_x _returnvalue_y) (`KismetMathLibrary.BreakVector2D` (`WidgetLayoutLibrary.GetViewportSize`)))
  (bind _screenlocation (`PlayerController.ProjectWorldLocationToScreen` (`GameplayStatics.GetPlayerController` 0) (`self.K2_GetActorLocation` (`Controller.K2_GetPawn` _returnvalue)) false))
  (`/Engine/EditorBlueprintResources/StandardMacros.IsValid` _returnvalue
    (:`Is Valid`
      (return (and (> (`KismetMathLibrary.BreakVector2D` _screenlocation) 0.0) (> (`.Y` (`KismetMathLibrary.BreakVector2D` _screenlocation)) 0.0) (< (`KismetMathLibrary.BreakVector2D` _screenlocation) _returnvalue_x) (< (`.Y` (`KismetMathLibrary.BreakVector2D` _screenlocation)) _returnvalue_y))))))

(fn `Set Spring Arm Length Basic`
  (params (Distance :type "Float (double-precision)"))
  (bind _springarm (`self.SpringArm`))
  (set `SpringArmComponent.TargetArmLength` (`KismetMathLibrary.FInterpTo` (`SpringArmComponent.TargetArmLength` _springarm) (`KismetMathLibrary.FClamp` (* (`self.SpringArmA`) Distance) (`self.MinCameraDistance`) (`self.MaxCameraDistance`)) (`GameplayStatics.GetWorldDeltaSeconds`) (`self.SprimArmInterpSpeed`)) _springarm))

(fn `SetCameraTransform2P`
  (bind (_returnvalue_x _returnvalue_y) (`KismetMathLibrary.BreakVector` (`self.K2_GetActorLocation` (`self.Player1`))))
  (bind (_returnvalue_x_2 _returnvalue_y_2) (`KismetMathLibrary.BreakVector` (`self.K2_GetActorLocation` (`self.Player2`))))
  (`self.SetCameraTransformBasic` (/ (+ _returnvalue_x _returnvalue_x_2) 2.0) (/ (+ _returnvalue_y _returnvalue_y_2) 2.0)))

(fn `SetCameraTransform3P`
  (bind (_returnvalue_x _returnvalue_y) (`KismetMathLibrary.BreakVector` (`self.K2_GetActorLocation` (`self.Player1`))))
  (bind (_returnvalue_x_2 _returnvalue_y_2) (`KismetMathLibrary.BreakVector` (`self.K2_GetActorLocation` (`self.Player3`))))
  (bind (_returnvalue_x_3 _returnvalue_y_3) (`KismetMathLibrary.BreakVector` (`self.K2_GetActorLocation` (`self.Player2`))))
  (`self.SetCameraTransformBasic` (/ (+ _returnvalue_x _returnvalue_x_3 _returnvalue_x_2) 3.0) (/ (+ _returnvalue_y _returnvalue_y_3 _returnvalue_y_2) 3.0)))

(fn `SetCameraTransform4P`
  (bind (_returnvalue_x _returnvalue_y) (`KismetMathLibrary.BreakVector` (`self.K2_GetActorLocation` (`self.Player3`))))
  (bind (_returnvalue_x_2 _returnvalue_y_2) (`KismetMathLibrary.BreakVector` (`self.K2_GetActorLocation` (`self.Player1`))))
  (bind (_returnvalue_x_3 _returnvalue_y_3) (`KismetMathLibrary.BreakVector` (`self.K2_GetActorLocation` (`self.Player4`))))
  (bind (_returnvalue_x_4 _returnvalue_y_4) (`KismetMathLibrary.BreakVector` (`self.K2_GetActorLocation` (`self.Player2`))))
  (`self.SetCameraTransformBasic` (/ (+ _returnvalue_x_2 _returnvalue_x_4 _returnvalue_x _returnvalue_x_3) 4.0) (/ (+ _returnvalue_y_2 _returnvalue_y_4 _returnvalue_y _returnvalue_y_3) 4.0)))

(fn `SetCameraTransformBasic`
  (params (X :type "Float (double-precision)") (Y :type "Float (double-precision)"))
  (bind _camera (`self.Camera`))
  (`SceneComponent.K2_SetWorldRotation` (`self.Camera`) (`KismetMathLibrary.RInterpTo` (`SceneComponent.K2_GetComponentRotation` _camera) (`KismetMathLibrary.FindLookAtRotation` (`SceneComponent.K2_GetComponentLocation` _camera) (`KismetMathLibrary.MakeVector` X Y)) (`GameplayStatics.GetWorldDeltaSeconds`) (`self.RotationInterpSpeed`)) false false)
  (`self.K2_SetActorLocation` (`KismetMathLibrary.VInterpTo` (`self.K2_GetActorLocation`) (`KismetMathLibrary.MakeVector` (`KismetMathLibrary.FClamp` X (`self.xCameraMinLimit`) (`self.xCameraMaxLimit`)) (`KismetMathLibrary.FClamp` Y (`self.yCameraMinLimit`) (`self.yCameraMaxLimit`))) (`GameplayStatics.GetWorldDeltaSeconds`) (`self.TransformInterpSpeed`))))

(fn `SetSpringArmLength2P`
  (`self.Set Spring Arm Length Basic` (`self.GetDistanceTo` (`self.Player1`) (`self.Player2`))))

(fn `SetSpringArmLength3P`
  (bind _player1 (`self.Player1`))
  (bind _player2 (`self.Player2`))
  (bind _player3 (`self.Player3`))
  (`self.Set Spring Arm Length Basic` (`.MaxValue` (`KismetMathLibrary.MaxOfFloatArray` (`|MakeArray` (`self.GetDistanceTo` _player1 _player2) (`self.GetDistanceTo` _player1 _player3) (`self.GetDistanceTo` _player2 _player3))))))

(fn `SetSpringArmLength4P`
  (bind _player1 (`self.Player1`))
  (bind _player2 (`self.Player2`))
  (bind _player3 (`self.Player3`))
  (bind _player4 (`self.Player4`))
  (`self.Set Spring Arm Length Basic` (`.MaxValue` (`KismetMathLibrary.MaxOfFloatArray` (`|MakeArray` (`self.GetDistanceTo` _player1 _player2) (`self.GetDistanceTo` _player1 _player3) (`self.GetDistanceTo` _player1 _player4) (`self.GetDistanceTo` _player2 _player3) (`self.GetDistanceTo` _player2 _player4) (`self.GetDistanceTo` _player3 _player4))))))

(fn `UserConstructionScript`)