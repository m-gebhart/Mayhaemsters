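; BP_Swayable is a prop actor, an umbrella or palm tree chosen by Type in the construction script, that sways when Sway is triggered.
; Sway picks random X/Y tilt offsets within set ranges and plays the SwayMotion timeline, stopping it after two seconds.
; The timeline lerps the root's world rotation from the BeginPlay rotation toward that tilt, ping-ponging by reversing or replaying on each finish.
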(event `self.ReceiveBeginPlay`
  (set `self.OriginalRot` (`self.K2_GetActorRotation`)))

(event `SwayPlay`
  (bind _originalrot (`self.OriginalRot`))
  (bind (_direction _rotation) (`Timeline|SwayMotion` :!label _label)
    (:`Update`
      (`SceneComponent.K2_SetWorldRotation` (`self.DefaultSceneRoot`) (`KismetMathLibrary.RLerp` _originalrot (`KismetMathLibrary.MakeRotator` (+ (.roll _originalrot) (`KismetMathLibrary.Conv_IntToDouble` (`self.RandRotX`))) (+ (.pitch _originalrot) (`KismetMathLibrary.Conv_IntToDouble` (`self.RandRotY`))) (.yaw _originalrot)) _rotation true) false false))
    (:`Finished`
      (if (`|EnumEquality` _direction "Forward")
        (`self.SwayReverse`)
        (else
          (`self.SwayPlay`))))))

(event `Sway`
  (`|ExecutionSequence`
    (:`then_0`
      (set `self.RandRotX` (`KismetMathLibrary.RandomIntegerInRange` (`self.XMin`) (`self.XMax`)))
      (set `self.RandRotY` (`KismetMathLibrary.RandomIntegerInRange` (`self.YMin`) (`self.YMax`)))
      (goto _label))
    (:`then_1`
      (`KismetSystemLibrary.Delay` 2.0)
      (goto _label :!via `Stop`))))

(event `SwayReverse`
  (goto _label :!via `Reverse`))

(fn `UserConstructionScript`
  (bind _staticmesh (`self.StaticMesh`))
  (switch `/Game/Blueprints/Miscellaneous/E_SwayableType` (`self.Type`)
    (:`NewEnumerator0`
      (`StaticMeshComponent.SetStaticMesh` _staticmesh "/Game/Meshes/StaticMeshes/Umbrella/StM_Umbrella.StM_Umbrella"))
    (:`NewEnumerator1`
      (`StaticMeshComponent.SetStaticMesh` _staticmesh "/Game/Meshes/LPStylizedEnv/Prototyping/Meshes/Trees/StM_PalmTree.StM_PalmTree"))))