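; BP_Extinguishable is a fire prop with a light, set up as a totem or campfire in the construction script.
; When AAQuality is above zero, it binds to the game state's environment-change event.
; That event hides flagged fires and lights after a short delay, then reignites them after a random wait unless the map is resetting.
; BeginPlay also scales light intensity by the game mode's time of day.
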(event `IgniteFire`
  (if (not (`C_GS_Mayhaemsters.bIsResettingMap` (`self.GameStateRef`)))
    (`SceneComponent.SetVisibility` (`self.Light`) true false)
    (`SceneComponent.SetVisibility` (`self.Fire`) true false)))

(event `ExtiguishFire`
  (if (`self.bShouldBeExtinguished`)
    (`KismetSystemLibrary.Delay` 0.6)
    (`SceneComponent.SetVisibility` (`self.Light`) false false)
    (`SceneComponent.SetVisibility` (`self.Fire`) false false)
    (`KismetSystemLibrary.Delay` (`KismetMathLibrary.RandomFloatInRange` 6.0 10.0))
    (`self.IgniteFire`)))

(event `self.ReceiveBeginPlay`
  (bind _light (`self.Light`))
  (bind _timeofday (`C_GM_Mayhaemsters.TimeOfDay` (cast `/Game/Blueprints/Game/BP_GM_Mayhaemsters` (`GameplayStatics.GetGameMode`) :!pure true)))
  (`|ExecutionSequence`
    (:`then_0`
      (bind _output_get (set `self.GameStateRef` (cast `/Game/Blueprints/Game/BP_GS_Mayhaemsters` (`GameplayStatics.GetGameState`) :!pure true)))
      (if (> (`C_GI_Mayhaemsters.AAQuality` (cast `/Game/Blueprints/Game/BP_GI_Mayhaemsters` (`GameplayStatics.GetGameInstance`) :!pure true)) 0)
        (add `/Game/Blueprints/Game/BP_GS_Mayhaemsters.ChangeEnvironment` _output_get (delegate `ExtiguishFire`))))
    (:`then_1`
      ;[1 1 1] set intensity
      (`KismetSystemLibrary.Delay` 0.05)
      (`LocalLightComponent.SetIntensityUnits` _light "Candelas")
      (if (`|EnumEquality` _timeofday "Day")
        (`LightComponent.SetIntensity` _light 50.0)
        (elif (`|EnumEquality` _timeofday "Dusk")
          (`LightComponent.SetIntensity` _light 120.0)
          (else
            (`LightComponent.SetIntensity` _light 160.0)))))))

(fn `UserConstructionScript`
  (bind _type (`self.Type`))
  (bind _staticmesh (`self.StaticMesh`))
  (bind _fire (`self.Fire`))
  (bind _staticmesh_2 (`self.StaticMesh`))
  (bind _fire_2 (`self.Fire`))
  (if (`|EnumEquality` _type "NewEnumerator0")
    (`StaticMeshComponent.SetStaticMesh` _staticmesh "/Game/Meshes/StaticMeshes/Totem/totem.totem")
    (`SceneComponent.K2_SetRelativeLocation` _fire_2 (0.0 0.0 344.0) false false)
    (`SceneComponent.SetRelativeScale3D` _fire (2.0 2.0 2.0))
    (`SceneComponent.SetRelativeScale3D` _staticmesh_2 (1.0 1.0 1.0))
    (elif (`|EnumEquality` _type "NewEnumerator1")
      (`StaticMeshComponent.SetStaticMesh` _staticmesh "/Game/Meshes/LPStylizedEnv/Prototyping/Meshes/CampTools/StM_CampFire.StM_CampFire")
      (`SceneComponent.K2_SetRelativeLocation` _fire_2 (0.0 0.0 180.0) false false)
      (`SceneComponent.SetRelativeScale3D` _fire (3.5 3.5 3.5))
      (`SceneComponent.SetRelativeScale3D` _staticmesh_2 (3.5 3.5 3.5)))))