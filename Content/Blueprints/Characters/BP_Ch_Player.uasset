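; Player character for Mayhaemsters: a hamster with a paper plane, colored by player index for up to four players.
; Tick runs one-time coloring and death, and syncs shield, slow smoke and attack animation to state flags.
; Events forward item UI to the GameState, sway world meshes and spawn timed dash ghosts.
; Death triggers an explosion and drops a timeline-driven grave that can self-destruct overlapping players; hover logic is unwired.
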(event `self.ActivateMystery`
  (params (PlayerID :type Integer))
  ;[1 1 1] items UI
  (`/Game/Blueprints/Game/BP_GS_Mayhaemsters.MystifyUI` (cast `/Game/Blueprints/Game/BP_GS_Mayhaemsters` (`GameplayStatics.GetGameState`) :!pure true) PlayerID))

(event `self.UpdateUnifierUI`
  (params (PlayerID :type Integer) (UnifiedButton :type Integer))
  ;[1 1 1] items UI
  (`/Game/Blueprints/Game/BP_GS_Mayhaemsters.UnifyUI` (cast `/Game/Blueprints/Game/BP_GS_Mayhaemsters` (`GameplayStatics.GetGameState`) :!pure true) PlayerID UnifiedButton))

(event `self.UpdateJammerUI`
  (params (PlayerID :type Integer) (JammedButtons :type "Array of Integer (by ref)"))
  ;[1 1 1] items UI
  (`/Game/Blueprints/Game/BP_GS_Mayhaemsters.JammerUI` (cast `/Game/Blueprints/Game/BP_GS_Mayhaemsters` (`GameplayStatics.GetGameState`) :!pure true) PlayerID JammedButtons))

(event `self.ReceiveTick`
  (params (DeltaSeconds :type "Float (single-precision)"))
  (bind _shield (`self.shield`))
  (bind _p_smoke (`self.P_Smoke`))
  (bind _binattackanimation (`self.bInAttackAnimation`))
  ;[1 1 1] Tick
  (`|ExecutionSequence`
    (:`then_0`
      (if (not (`self.bInstantiated`))
        (`self.SetColor`)))
    (:`then_1`
      (if (`self.bIsDead`)
        (if (not (`self.DeadAnimInstantiated`))
          (`self.DeathScript`)
          (set `self.DeadAnimInstantiated` true))
        (else
          (`|ExecutionSequence`
            (:`then_0`
              (if (`self.bIsShieldActive`)
                (`SceneComponent.SetVisibility` _shield true false)
                (else
                  (`SceneComponent.SetVisibility` _shield false false))))
            (:`then_1`
              (if (`self.bIsSlowed`)
                (`SceneComponent.SetVisibility` _p_smoke true false)
                (else
                  (`SceneComponent.SetVisibility` _p_smoke false false))))
            (:`then_2`
              (bind _asanim_bp_hamster (cast `/Game/Meshes/SkeletalMeshes/Hamster/AnimBP_Hamster` (`SkeletalMeshComponent.GetAnimInstance` (`self.Mesh`))))
              (if (`self.bCanShoot`)
                (if _binattackanimation
                  (set `/Game/Meshes/SkeletalMeshes/Hamster/AnimBP_Hamster.Idle_Attack` 0.0 _asanim_bp_hamster)
                  (set `self.bInAttackAnimation` false))
                (elif (not _binattackanimation)
                  (set `self.bInAttackAnimation` true)
                  (if (== (`/Game/Meshes/SkeletalMeshes/Hamster/AnimBP_Hamster.Idle_Attack` _asanim_bp_hamster) 0.0)
                    (set `/Game/Meshes/SkeletalMeshes/Hamster/AnimBP_Hamster.Idle_Attack` 100.0 _asanim_bp_hamster)))))))))))

(event `self.ReceiveBeginPlay`
  ;[1 1 1] BeginPlay
  (set `self.GameModeRef` (cast `/Game/Blueprints/Game/BP_GM_Mayhaemsters` (`GameplayStatics.GetGameMode`) :!pure true)))

(event `self.SwayWorldMesh`
  (params (HitActor :type "Actor Object Reference"))
  ;[1 1 1] sway mesh
  (bind _asbp_swayable (cast `/Game/Blueprints/Actors/BP_Swayable` HitActor))
  (`/Game/Blueprints/Actors/BP_Swayable.Sway` _asbp_swayable))

(event `self.ShowDashGhost`
  (params (PlayerID :type Integer))
  ;[1 1 1] show ghost
  (`ParticleSystemComponent.BeginTrails` (`self.AnimTrails`) "Neck" "Head" "ETrailWidthMode_FromCentre" 10.0)
  (bind _returnvalue (`KismetSystemLibrary.K2_SetTimerDelegate` (delegate `ShowGhost`) 0.1 true))
  (bind _asbp_ch_player (cast `/Game/Blueprints/Characters/BP_Ch_Player` (`GameplayStatics.GetPlayerCharacter` PlayerID)))
  (bind _animtrails (`/Game/Blueprints/Characters/BP_Ch_Player.AnimTrails` _asbp_ch_player))
  (bind _returnvalue_2 (`PrimitiveComponent.CreateDynamicMaterialInstance` _animtrails 0 (`PrimitiveComponent.GetMaterial` _animtrails 0) "None"))
  (`MaterialInstanceDynamic.SetVectorParameterValue` _returnvalue_2 "TrailColor" (struct :`R` 0.6875 :`G` 0.6875 :`B` 0.6875 :`A` 1.0)))

(event `ShowGhost`
  ;[1 1 1] show ghost
  (`|SpawnActorFromClass` "/Game/Blueprints/Actors/BP_GhostTrails.BP_GhostTrails_C" (`SceneComponent.K2_GetComponentToWorld` (`self.Mesh`)) "Undefined" "OverrideRootScale" null null)
  (if (not (`self.bIsDashing`))
    (`KismetSystemLibrary.K2_ClearAndInvalidateTimerHandle` (stale `self.ShowDashGhost` _returnvalue))
    (`ParticleSystemComponent.EndTrails` (`self.AnimTrails`))))

(event `SpawnGrave`
  (bind _returnvalue (+ (`self.K2_GetActorLocation`) (`KismetMathLibrary.MakeVector` (`KismetMathLibrary.RandomFloatInRange` 150.0 250.0) (`KismetMathLibrary.RandomFloatInRange` 150.0 250.0) 7500.0)))
  ;[1 1 1] grave
  (bind _returnvalue_2 (`AddComponent|NODE_AddStaticMeshComponent-2`))
  (bind _returnvalue_3 (`AddComponent|NODE_AddSphereComponent-0` :`bManualAttachment` true))
  (set `self.GraveSphereCol` _returnvalue_3)
  (`SceneComponent.K2_AttachToComponent` _returnvalue_3 _returnvalue_2 "None" "SnapToTarget" "SnapToTarget" "SnapToTarget" true)
  (`SphereComponent.SetSphereRadius` _returnvalue_3 500.0 true)
  (bind _outhit (`KismetSystemLibrary.LineTraceSingleForObjects` _returnvalue (+ _returnvalue (0.0 0.0 -10000.0)) (`|MakeArray` "ObjectTypeQuery1" :!type "EObjectTypeQuery Enum")))
  (bind (_direction _gravez) (`Timeline|GraveFall` :!via `PlayFromStart`)
    (:`Update`
      (`SceneComponent.K2_SetWorldTransform` _returnvalue_2 (`KismetMathLibrary.MakeTransform` (`KismetMathLibrary.VLerp` _returnvalue (`.ImpactPoint` (`GameplayStatics.BreakHitResult` _outhit)) _gravez) (struct :`Yaw` 90.0 :`Roll` 90.0) (0.6 0.6 0.6)) false false)
      (`StaticMeshComponent.SetStaticMesh` _returnvalue_2 "/Game/Meshes/StaticMeshes/Grave/StM_Grave.StM_Grave")
      (`PrimitiveComponent.SetCollisionEnabled` _returnvalue_2 "NoCollision")
      (for _array_element (`/Game/Blueprints/Game/BP_GM_Mayhaemsters.AllPlayers` (`self.GameModeRef`))
        (if (and (`PrimitiveComponent.IsOverlappingActor` (`self.GraveSphereCol`) _array_element) (!= _array_element self))
          (`/Engine/EditorBlueprintResources/StandardMacros.DoOnce` false
            (:`Completed`
              (`self.SelfDestruct` _array_element)
              (`self.SetActorEnableCollision` false))))))))

(fn `DeathScript`
  (`GameplayStatics.SpawnEmitterAtLocation` "/Game/Particles/P_Explosion.P_Explosion" (+ (`self.K2_GetActorLocation` self) (0.0 0.0 50.0)) (struct) (7.0 7.0 7.0))
  (for _array_element (`|MakeArray` (`self.plane`) (`self.shield`))
    (`/Engine/EditorBlueprintResources/StandardMacros.IsValid` _array_element
      (:`Is Valid`
        (`SceneComponent.SetVisibility` _array_element false false)
        (`PrimitiveComponent.SetCollisionEnabled` _array_element "NoCollision"))))
  (`SceneComponent.SetVisibility` (`self.Mesh`) false false)
  (`self.SpawnGrave`))

(fn `SetColor`
  (bind _playerindex (`self.PlayerIndex`))
  (bind _asbp_gi_mayhaemsters (cast `/Game/Blueprints/Game/BP_GI_Mayhaemsters` (`GameplayStatics.GetGameInstance`)))
  (if (> (`C_GI_Mayhaemsters.PlayerCount` _asbp_gi_mayhaemsters) _playerindex)
    (bind _asbp_pc_player (cast `/Game/Blueprints/Characters/BP_PC_Player` (`GameplayStatics.GetPlayerController` _playerindex)))
    (set `self.bInstantiated` true)
    (bind _asbp_ch_player (cast `/Game/Blueprints/Characters/BP_Ch_Player` (`Controller.K2_GetPawn` _asbp_pc_player)))
    (bind _returnvalue (`PrimitiveComponent.CreateDynamicMaterialInstance` (`Character.Mesh` _asbp_ch_player) 0 null "None"))
    (switch `int` _playerindex
      (:`0`
        (`MaterialInstanceDynamic.SetTextureParameterValue` _returnvalue "Param" "/Game/Meshes/SkeletalMeshes/Hamster/Textures/Hamster/M_Hamster_Blue.M_Hamster_Blue"))
      (:`1`
        (`MaterialInstanceDynamic.SetTextureParameterValue` _returnvalue "Param" "/Game/Meshes/SkeletalMeshes/Hamster/Textures/Hamster/M_Hamster_Orange.M_Hamster_Orange"))
      (:`2`
        (`MaterialInstanceDynamic.SetTextureParameterValue` _returnvalue "Param" "/Game/Meshes/SkeletalMeshes/Hamster/Textures/Hamster/M_Hamster_Purple.M_Hamster_Purple"))
      (:`3`
        (`MaterialInstanceDynamic.SetTextureParameterValue` _returnvalue "Param" "/Game/Meshes/SkeletalMeshes/Hamster/Textures/Hamster/M_Hamster_Green.M_Hamster_Green")))
    (`PrimitiveComponent.SetMaterial` (`self.plane`) 0 "/Game/Meshes/StaticMeshes/Plane/M_PaperPlane.M_PaperPlane")))

(fn `UserConstructionScript`)