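; Game instance for Mayhaemsters that builds the list of selectable screen resolutions and applies the highest one.
; GetAvailableResolutions keeps supported fullscreen resolutions with an exact 16:9 ratio in AvailableResolutions, then calls SetHighestResolution and records the last index as current.
; SetHighestResolution treats the last entry as the highest and applies it through an r.SetRes console command suffixed with FullScreenState.
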(event `GetAvailableResolutions`
  (bind _resolutionindex (`self.ResolutionIndex`))
  (`|ExecutionSequence`
    (:`then_0`
      (bind _resolutions (`KismetSystemLibrary.GetSupportedFullscreenResolutions`))
      (for _array_element _resolutions
        (bind (_x _y) (break `IntPoint` _array_element))
        (if (== (/ (`KismetMathLibrary.Conv_IntToDouble` _x) (`KismetMathLibrary.Conv_IntToDouble` _y)) (/ 16.0 9.0))
          (`KismetArrayLibrary.Array_Set` (`self.AvailableResolutions`) _resolutionindex _array_element true)
          (`/Engine/EditorBlueprintResources/StandardMacros.IncrementInt` _resolutionindex))))
    (:`then_1`
      (`self.SetHighestResolution`))
    (:`then_2`
      (set `self.CurrentScreenResolutionIndex` (`KismetArrayLibrary.Array_LastIndex` (`self.AvailableResolutions`))))))

(event `SetHighestResolution`
  (bind _availableresolutions (`self.AvailableResolutions`))
  (bind (_x _y) (break `IntPoint` (`|GetArrayItem` _availableresolutions (`KismetArrayLibrary.Array_LastIndex` _availableresolutions))))
  (`KismetSystemLibrary.ExecuteConsoleCommand` (`KismetStringLibrary.Concat_StrStr` "r.SetRes " (`KismetStringLibrary.Conv_IntToString` _x) "x" (`KismetStringLibrary.Conv_IntToString` _y) (`self.FullScreenState`)) (`GameplayStatics.GetPlayerController` 0)))