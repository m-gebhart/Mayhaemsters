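; Game state for Mayhaemsters that runs a rising and falling sea whenever the map reset event fires.
; A timeline lifts the SeaMesh-tagged static mesh to the final level, pauses briefly, then reverses and clears the resetting flag.
; During movement it flags Grave-tagged players as grounded; the code that sinks them is disconnected.
; A DoOnce plays the reset sound and calls the environment change once per cycle.
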(event `self.ReceiveBeginPlay`
  ;[1 1 1] raise and lower the sea level when the map resetter is used
  (add `self.OnMapReset` self (delegate `RaiseSeaLevel`))
  (bind _outactors (`GameplayStatics.GetAllActorsOfClassWithTag` "/Script/Engine.StaticMeshActor" "SeaMesh"))
  (for _array_element _outactors
    (bind _output_get (set `self.SeaMesh` _array_element))
    (set `self.InitialSeaLevel` (`self.K2_GetActorLocation` _output_get))))

(event `RaiseSeaLevel`
  (bind _initialsealevel (`self.InitialSeaLevel`))
  ;[1 1 1] raise and lower the sea level when the map resetter is used
  (bind (_direction _alpha) (`Timeline|Raise/LowerSea` :!via `PlayFromStart` :!label _label)
    (:`Update`
      (`self.K2_SetActorLocation` (`self.SeaMesh`) (`KismetMathLibrary.VLerp` _initialsealevel (`KismetMathLibrary.MakeVector` (.x _initialsealevel) (.y _initialsealevel) (`self.FinalSeaLevel`)) _alpha) false false)
      (`self.RemoveGraves`)
      (`/Engine/EditorBlueprintResources/StandardMacros.DoOnce` false :!label _label_2
        (:`Completed`
          (`GameplayStatics.PlaySound2D` "/Game/Audio/SoundCues/ResetMapSoundCue.ResetMapSoundCue" 1.0 1.0 0.0 null null)
          (`self.ChangeEnvironment`))))
    (:`Finished`
      (if (`|EnumEquality` _direction "Forward")
        (`KismetSystemLibrary.Delay` 0.5)
        (`self.LowerSeaLevel`)
        (goto _label_2 :!via `Reset`)
        (else
          (set `self.bIsResettingMap` false)
          (goto _label_2 :!via `Reset`))))))

(event `LowerSeaLevel`
  ;[1 1 1] raise and lower the sea level when the map resetter is used
  (goto _label :!via `ReverseFromEnd`))

(fn `RemoveGraves`
  (bind _outactors (`GameplayStatics.GetAllActorsOfClassWithTag` "/Game/Blueprints/Characters/BP_Ch_Player.BP_Ch_Player_C" "Grave"))
  (for _array_element _outactors
    (bind _asbp_ch_player (cast `/Game/Blueprints/Characters/BP_Ch_Player` _array_element))
    (if (not (`C_Ch_Player.bGraveGrounded` _asbp_ch_player))
      (set `C_Ch_Player.bGraveGrounded` true _asbp_ch_player))))

(fn `UserConstructionScript`)