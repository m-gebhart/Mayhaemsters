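; Game mode for Mayhaemsters that creates the in-game UI, starts beach ambience, spawns pickups and switches time-of-day lighting.
; A looping timer spawns randomly typed pickups at tagged target points while fewer than five exist, tracking point availability by index and recursively retrying when a chosen point is occupied.
; SetDayTime finds the tagged sun and the skylight, then applies Day, Dusk or Night presets through SetSunProperties.
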(event `self.SetDayTime`
  (params (DayTime :type "ETimeOfDay Enum" :default "Day"))
  ;[1 1 1] time of day
  (`KismetSystemLibrary.Delay` 0.05)
  (`|ExecutionSequence`
    (:`then_0`
      (bind _outactors (`GameplayStatics.GetAllActorsOfClassWithTag` "/Script/Engine.DirectionalLight" "Sun"))
      (for _array_element _outactors
        (bind _asdirectional_light (cast `DirectionalLight` _array_element))
        (set `self.SunRef` _asdirectional_light)))
    (:`then_1`
      (bind _outactors_2 (`GameplayStatics.GetAllActorsOfClass` "/Script/Engine.SkyLight"))
      (for _array_element_2 _outactors_2
        (set `self.SkyRef` _array_element_2)))
    (:`then_2`
      (switch `ETimeOfDay` DayTime
        (:`Day`
          (`self.SetSunProperties` (struct :`Pitch` -61.0 :`Yaw` 466.0 :`Roll` 263.0) 7.0 (struct :`R` 1.0 :`G` 0.737255 :`B` 0.219608 :`A` 1.0) 1.0))
        (:`Dusk`
          (`self.SetSunProperties` (struct :`Pitch` -30.0 :`Yaw` 540.0 :`Roll` 270.0) 5.0 (struct :`R` 0.47451 :`G` 0.34902 :`B` 0.101961 :`A` 1.0) 0.5))
        (:`Night`
          (`self.SetSunProperties` (struct :`Pitch` 24.0 :`Yaw` 475.0 :`Roll` 130.0) 0.0 (struct :`R` 0.129412 :`G` 0.094118 :`B` 0.027451 :`A` 1.0) -5.0))))))

(event `self.ReceiveBeginPlay`
  (`|ExecutionSequence`
    (:`then_0`
      (bind _returnvalue (`|CreateWidget` "/Game/Blueprints/Widgets/WBP_InGameUI.WBP_InGameUI_C" (`GameplayStatics.GetPlayerController` 0)))
      (bind _output_get (set `self.InGameUI` _returnvalue))
      (`UserWidget.AddToViewport` _output_get 0)
      (`GameplayStatics.PlaySoundAtLocation` "/Game/Audio/SoundCues/Beach_Theme_v1_0_Cue.Beach_Theme_v1_0_Cue" (0.0 0.0 0.0) (struct) 1.0 1.0 0.0 null null null)
      (`GameplayStatics.PlaySoundAtLocation` "/Game/Audio/SoundCues/Waves.Waves" (0.0 0.0 0.0) (struct) 1.0 1.0 0.0 null null null)
      (`GameplayStatics.PlaySoundAtLocation` null (0.0 0.0 0.0) (struct) 1.0 1.0 0.0 null null null))
    (:`then_1`
      ;[1 1 1] spawning items
      (bind _outactors (`GameplayStatics.GetAllActorsOfClassWithTag` "/Script/Engine.TargetPoint" "ItemSpawnLoc"))
      (bind _output_get_2 (set `self.ItemSpawnPoints` _outactors))
      (for (_ _array_index) _output_get_2
        (`KismetArrayLibrary.Array_Set` (`self.SpawnPointAvailability`) _array_index true true)))
    (:`then_2`
      (if (> (`KismetArrayLibrary.Array_Length` (`self.ItemSpawnPoints`)) 0)
        (`KismetSystemLibrary.K2_SetTimerDelegate` (delegate `SpawnItems`) (`self.ItemSpawnInterval`) true)))
    (:`then_3`
      (`KismetSystemLibrary.Delay` 0.05)
      (bind _outactors_2 (`GameplayStatics.GetAllActorsOfClass` "/Game/Blueprints/Characters/BP_Ch_Player.BP_Ch_Player_C"))
      (set `self.AllPlayers` _outactors_2))))

(event `SpawnItems`
  (bind (_returnvalue_roll _returnvalue_pitch _returnvalue_yaw) (`KismetMathLibrary.BreakRotator` (`KismetMathLibrary.RandomRotator` false)))
  (bind _numberofavailablespawnpoints (`self.NumberOfAvailableSpawnPoints`))
  (bind _randomspawnpointindex (`self.RandomSpawnPointIndex`))
  (bind _spawnpointavailability (`self.SpawnPointAvailability`))
  ;[1 1 1] spawning items
  (bind _outactors (`GameplayStatics.GetAllActorsOfClass` "/Game/Blueprints/Actors/BP_PickupItem.BP_PickupItem_C"))
  (set `self.RandomSpawnPointIndex` (`KismetMathLibrary.RandomIntegerInRange` 0 (`KismetArrayLibrary.Array_LastIndex` (`self.ItemSpawnPoints`))))
  (if (< (`KismetArrayLibrary.Array_Length` _outactors) 5)
    (if (`|GetArrayItem` _spawnpointavailability _randomspawnpointindex)
      (`KismetArrayLibrary.Array_Set` _spawnpointavailability _randomspawnpointindex)
      (bind _returnvalue (`|SpawnActorFromClass` "/Game/Blueprints/Actors/BP_PickupItem.BP_PickupItem_C" (`KismetMathLibrary.MakeTransform` (`self.K2_GetActorLocation` (`|GetArrayItem` (`self.ItemSpawnPoints`) _randomspawnpointindex)) (`KismetMathLibrary.MakeRotator` 0.0 0.0 _returnvalue_yaw)) "Undefined" "OverrideRootScale" null null))
      (bind _output_get (set `self.SpawnedItem` _returnvalue))
      (set `/Game/Blueprints/Actors/BP_PickupItem.ItemIndex` (`self.RandomSpawnPointIndex`) _output_get)
      (bind _returnvalue_2 (`self.GetItemTypeInt` (`KismetMathLibrary.RandomIntegerInRange` 0 100)))
      (set `C_PickupItem.ItemType` (cast `EPickupItemType` (`KismetMathLibrary.Conv_IntToByte` _returnvalue_2)) _output_get)
      (`/Game/Blueprints/Actors/BP_PickupItem.Set Item Mesh` _output_get)
      (else
        (set `self.NumberOfAvailableSpawnPoints` 0)
        (for _array_element (`self.SpawnPointAvailability`)
          (if _array_element
            (`|ExecutionSequence`
              (:`then_0`
                (`/Engine/EditorBlueprintResources/StandardMacros.IncrementInt` _numberofavailablespawnpoints))
              (:`then_1`
                (if (> _numberofavailablespawnpoints 0)
                  (`self.SpawnItems`))))))))))

(fn `SetSunProperties`
  (params (SunRotation :type "Rotator Structure") (SunIntensity :type "Float (double-precision)") (SunColor :type "LinearColor Structure") (SkyIntensity :type "Float (double-precision)"))
  (bind _sunref (`self.SunRef`))
  (bind _lightcomponent (`Light.LightComponent` _sunref))
  (`self.K2_SetActorRotation` _sunref SunRotation false)
  (`LightComponent.SetIntensity` _lightcomponent SunIntensity)
  (`LightComponent.SetLightColor` _lightcomponent SunColor true)
  (`SkyLightComponent.SetIntensity` (`SkyLight.LightComponent` (`self.SkyRef`)) SkyIntensity))

(fn `UserConstructionScript`)